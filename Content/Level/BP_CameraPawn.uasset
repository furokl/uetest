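; BP_CameraPawn is a spring-arm camera pawn that moves to focus on an actor the player clicks.
; A short delay after each press separates holds, which set ClickHeld, from clicks, which trace under the cursor on the Visibility channel.
; A blocking hit drives FocusTimeline, which lerps from the pawn's current location toward the focused actor each update.
; The construction script caches the default arm length, though nothing here reads it.
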(event `InputAction|Click`
  (params (Key :type "Key Structure"))
  (:`Pressed`
    (`KismetSystemLibrary.Delay` 0.2)
    (`self.HandleMouseClick` Key))
  (:`Released`
    (set `self.bClickHeld` false)))

(event `Move To FocusedActor`
  (params (FocusedActor :type "Actor Object Reference"))
  (bind (_direction _anim_timeline) (`Timeline|Focus Timeline`)
    (:`Update`
      (`self.K2_SetActorLocation` (`KismetMathLibrary.VLerp` (`self.K2_GetActorLocation`) (`self.K2_GetActorLocation` FocusedActor) _anim_timeline)))))

(fn `CheckClickHitActor`
  (returns (bBlockingHit :type Boolean) (HitActor :type "Actor Object Reference"))
  (bind (_bblockinghit _binitialoverlap _time _distance _location _impactpoint _normal _impactnormal _physmat _hitactor) (`GameplayStatics.BreakHitResult` (`PlayerController.GetHitResultUnderCursorByChannel` (`GameplayStatics.GetPlayerController` 0) "TraceTypeQuery1" true)))
  (return _bblockinghit _hitactor))

(fn `HandleMouseClick`
  (params (Key :type "Key Structure" :default "None"))
  (bind (_bblockinghit _hitactor) (`self.CheckClickHitActor`))
  (bind _returnvalue (`PlayerController.IsInputKeyDown` (`GameplayStatics.GetPlayerController` 0) Key))
  (if _returnvalue
    (set `self.bClickHeld` _returnvalue)
    (elif _bblockinghit
      (bind _output_get (set `self.FocusedActor` _hitactor))
      (`self.Move To FocusedActor` _output_get))))

(fn `UserConstructionScript`
  (set `self.DefaultArmLength` (`SpringArmComponent.TargetArmLength` (`self.SpringArm`))))